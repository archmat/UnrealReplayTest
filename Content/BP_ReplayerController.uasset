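; BP_ReplayerController is a player controller for replay viewing that owns the on-screen replay viewer UI.
; On BeginPlay it creates WID_ReplayViewer for the local controller, adds it to the viewport, and prints debug messages.
; After a replay time jump, it re-pauses playback if the widget's pause state is set, then refreshes the widget's pause button text.
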(event `self.ReceiveBeginPlay`
  (`KismetSystemLibrary.PrintString` (`KismetTextLibrary.Conv_TextToString` (`|FormatText` "BeginPlay : {PC} / Num : {num}" (`KismetSystemLibrary.GetDisplayName` (`GameplayStatics.GetPlayerController` 0)) (`GameplayStatics.GetNumPlayerControllers`))) true true (struct :`R` 0.775822 :`G` 0.304987 :`A` 1.0) 5.0)
  (if (`self.IsLocalPlayerController`)
    (bind _asbp_replayer_controller (cast `/Game/BP_ReplayerController` (`GameplayStatics.GetPlayerController` 0)))
    (bind _returnvalue (`|CreateWidget` "/Game/WID_ReplayViewer.WID_ReplayViewer_C" _asbp_replayer_controller))
    (`/Engine/EditorBlueprintResources/StandardMacros.IsValid` _returnvalue
      (:`Is Valid`
        (bind _output_get (set `self.ReplayViewerRef` _returnvalue))
        (`UserWidget.AddToViewport` _output_get 0))
      (:`Is Not Valid`
        (`KismetSystemLibrary.PrintString` "InValid : WID_ReplaySpectator" true true (struct :`R` 1.0 :`A` 1.0))))
    (else
      (`KismetSystemLibrary.PrintString` "Not Local Player Controller" true true (struct :`R` 1.0 :`A` 1.0)))))

(event `self.PostReplayGotoTime`
  (params (bWasSuccessful :type Boolean))
  (bind _replayviewerref (`self.ReplayViewerRef`))
  (`KismetSystemLibrary.PrintString` (`KismetStringLibrary.Conv_BoolToString` bWasSuccessful))
  (if (`/Game/WID_ReplayViewer.CurrentReplayPauseState` (`self.ReplayViewerRef`))
    (`self.PauseReplay`))
  (`/Engine/EditorBlueprintResources/StandardMacros.IsValid` _replayviewerref
    (:`Is Valid`
      (`/Game/WID_ReplayViewer.RefreshPauseButtonText` _replayviewerref))))

(fn `UserConstructionScript`)